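; Enemy actor that starts a battle with BP_Player on sphere overlap and resolves incoming attacks on three body emplacements: head, bust and belly.
; ChooseEmplacement shows the hitboxes and first hand marker, and ChangeIndex moves the visible marker.
; Damage routes AttackData to per-emplacement or AOE functions that rebuild EnnemyData, reducing shields and applying HP damage, doubled at the heart.
; Single-target functions loop per projectile and add through-shield and passive damage handling.
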(event `self.Sphere.OnComponentBeginOverlap`
  (params (OverlappedComponent :type "PrimitiveComponent Object Reference") (OtherActor :type "Actor Object Reference") (OtherComp :type "PrimitiveComponent Object Reference") (OtherBodyIndex :type Integer) (bFromSweep :type Boolean) (SweepResult :type "HitResult Structure (by ref)"))
  (if (not (`self.Move Player`))
    (bind _asbp_player (cast `/Game/GAME/BP/CHARACTER/BP_Player` OtherActor))
    (set `/Game/GAME/BP/CHARACTER/BP_Player.IsInBattle?` true _asbp_player)
    (bind _output_get (set `self.As BP Player` _asbp_player))
    (set `self.HimInBattle?` true)
    (`/Game/GAME/BP/CHARACTER/BP_Player.Start Battle` _output_get (`.ImpactPoint` (`GameplayStatics.BreakHitResult` SweepResult)))))

(event `/Game/GAME/BP/BPI/BPI_Ennemy_Interaction.Receive Damage`
  (params (Attack_Data :type "/Game/Structure/ST_Normal_Attack Structure"))
  (bind (_attackdamage _aoe_ _numberofprojectile _numberofshieldthatcanbebroken _candealdamagethroughshield_ _damageaddedperdestroyedshield _candealpassivedamage_ _passivedamage _targetedemplacement) (break `/Game/Structure/ST_Normal_Attack` Attack_Data))
  (bind (_pv _heartemplacement _nbrofshieldemplacement1 _nbrofshieldemplacement2 _nbrofshieldemplacement3) (break `/Game/Structure/ST_Ennemie_Data` (`self.Ennemy_Data`)))
  (if _aoe_
    (`self.All Emplacement Attaked` _numberofprojectile _attackdamage _numberofshieldthatcanbebroken _candealdamagethroughshield_ _damageaddedperdestroyedshield _candealpassivedamage_ _passivedamage _pv _heartemplacement _nbrofshieldemplacement1 _nbrofshieldemplacement2 _nbrofshieldemplacement3)
    (else
      (switch `int` _targetedemplacement
        (:`0`
          (`self.Emplacement 1 Attacked` _numberofprojectile _attackdamage _numberofshieldthatcanbebroken _candealdamagethroughshield_ _damageaddedperdestroyedshield _candealpassivedamage_ _passivedamage _pv _heartemplacement _nbrofshieldemplacement1 _nbrofshieldemplacement2 _nbrofshieldemplacement3))
        (:`1`
          (`self.Emplacement 2 Attacked` _numberofprojectile _attackdamage _numberofshieldthatcanbebroken _candealdamagethroughshield_ _damageaddedperdestroyedshield _candealpassivedamage_ _passivedamage _pv _heartemplacement _nbrofshieldemplacement1 _nbrofshieldemplacement2 _nbrofshieldemplacement3))
        (:`2`
          (`self.Emplacement 3 Attacked` _numberofprojectile _attackdamage _numberofshieldthatcanbebroken _candealdamagethroughshield_ _damageaddedperdestroyedshield _candealpassivedamage_ _passivedamage _pv _heartemplacement _nbrofshieldemplacement1 _nbrofshieldemplacement2 _nbrofshieldemplacement3)))))
  (`/Game/GAME/BP/CHARACTER/BP_Player.Attaque Anim` (`self.As BP Player`)))

(event `/Game/GAME/BP/BPI/BPI_Ennemy_Interaction.Choose Emplacement`
  (for _array_element (`self.HitBox Ref Array`)
    (`SceneComponent.SetVisibility` _array_element true false))
  (`SceneComponent.SetVisibility` (`|GetArrayItem` (`self.Hand Ref Array`)) true false))

(event `self.ReceiveBeginPlay`
  (bind _hitbox_ref_array (`self.HitBox Ref Array`))
  (bind _hand_ref_array (`self.Hand Ref Array`))
  (`KismetArrayLibrary.Array_Add` _hitbox_ref_array (`self.TeteHitbox`))
  (`KismetArrayLibrary.Array_Add` _hitbox_ref_array (`self.BusteHitbox`))
  (`KismetArrayLibrary.Array_Add` _hitbox_ref_array (`self.VentreHitBox`))
  (`KismetArrayLibrary.Array_Add` _hand_ref_array (`self.HandTete`))
  (`KismetArrayLibrary.Array_Add` _hand_ref_array (`self.HandBuste`))
  (`KismetArrayLibrary.Array_Add` _hand_ref_array (`self.HandBuste1`))
  (for _array_element (`self.Hand Ref Array`)
    (`SceneComponent.SetVisibility` _array_element false false))
  (for _array_element_2 (`self.HitBox Ref Array`)
    (`SceneComponent.SetVisibility` _array_element_2 false false)))

(event `Satin Blood`
  (bind _bloodstain (`self.BloodStain`))
  (`ActorComponent.Activate` _bloodstain false)
  (`KismetSystemLibrary.Delay` 0.2)
  (`ActorComponent.Deactivate` _bloodstain))

(event `/Game/GAME/BP/BPI/BPI_Ennemy_Interaction.ChangeIndex`
  (params (`Up?z` :type Boolean))
  (bind _hand_ref_array (`self.Hand Ref Array`))
  (if `Up?z`
    (set `self.EmplacmentAiming` (`KismetMathLibrary.Clamp` (- (`self.EmplacmentAiming`) 1) 0 2))
    (else
      (set `self.EmplacmentAiming` (`KismetMathLibrary.Clamp` (+ (`self.EmplacmentAiming`) 1) 0 2))))
  (for _array_element _hand_ref_array
    (`SceneComponent.SetVisibility` _array_element false false))
  (`SceneComponent.SetVisibility` (`|GetArrayItem` _hand_ref_array (`self.EmplacmentAiming`)) true false))

(fn `All Emplacement Attaked`
  (params (`Number Of Projectile` :type Integer) (`Native Damage` :type Integer) (`Number Of Shield That Can Be Broken` :type Integer) (`Can deal damage through shield ?` :type Boolean) (` Damage added per destroyed shield` :type Integer) (`Can Deal Passive Damage ?` :type Boolean) (`Passive Damage` :type Integer) (`Ennemy HP` :type Integer) (`Ennemy Heart Emplacement` :type Integer) (`Nbr Of Shield (Emplacement 1)` :type Integer) (`Nbr Of Shield (Emplacement 2)` :type Integer) (`Nbr Of Shield (Emplacement 3)` :type Integer))
  (bind _pv (break `/Game/Structure/ST_Ennemie_Data` (`self.Ennemy_Data`)))
  (bind _returnvalue (`KismetMathLibrary.Clamp` (- `Nbr Of Shield (Emplacement 3)` `Number Of Shield That Can Be Broken`) 0 5))
  (bind _returnvalue_2 (`KismetMathLibrary.Clamp` (- `Nbr Of Shield (Emplacement 1)` `Number Of Shield That Can Be Broken`) 0 5))
  (bind _returnvalue_3 (`KismetMathLibrary.Clamp` (- `Nbr Of Shield (Emplacement 2)` `Number Of Shield That Can Be Broken`) 0 5))
  (`|ExecutionSequence`
    (:`then_0`
      (if (== _returnvalue_2 0)
        (if (== `Ennemy Heart Emplacement` 0)
          (`KismetSystemLibrary.PrintString` "Critique")
          (set `self.Ennemy_Data` (make `/Game/Structure/ST_Ennemie_Data` (- `Ennemy HP` (* `Native Damage` 2)) `Ennemy Heart Emplacement` _returnvalue_2 `Nbr Of Shield (Emplacement 2)` `Nbr Of Shield (Emplacement 3)`))
          (else
            (`KismetSystemLibrary.PrintString` "Normal")
            (set `self.Ennemy_Data` (make `/Game/Structure/ST_Ennemie_Data` (- `Ennemy HP` `Native Damage`) `Ennemy Heart Emplacement` _returnvalue_2 `Nbr Of Shield (Emplacement 2)` `Nbr Of Shield (Emplacement 3)`))))
        (else
          (set `self.Ennemy_Data` (make `/Game/Structure/ST_Ennemie_Data` `Ennemy HP` `Ennemy Heart Emplacement` _returnvalue_2 `Nbr Of Shield (Emplacement 2)` `Nbr Of Shield (Emplacement 3)`)))))
    (:`then_1`
      (if (== _returnvalue_3 0)
        (if (== `Ennemy Heart Emplacement` 1)
          (`KismetSystemLibrary.PrintString` "Critique")
          (set `self.Ennemy_Data` (make `/Game/Structure/ST_Ennemie_Data` (- _pv (* `Native Damage` 2)) `Ennemy Heart Emplacement` `Nbr Of Shield (Emplacement 1)` _returnvalue_3 `Nbr Of Shield (Emplacement 3)`))
          (else
            (`KismetSystemLibrary.PrintString` "Normal")
            (set `self.Ennemy_Data` (make `/Game/Structure/ST_Ennemie_Data` (- _pv `Native Damage`) `Ennemy Heart Emplacement` `Nbr Of Shield (Emplacement 1)` _returnvalue_3 `Nbr Of Shield (Emplacement 3)`))))
        (else
          (set `self.Ennemy_Data` (make `/Game/Structure/ST_Ennemie_Data` _pv `Ennemy Heart Emplacement` `Nbr Of Shield (Emplacement 1)` _returnvalue_3 `Nbr Of Shield (Emplacement 3)`)))))
    (:`then_2`
      (if (== _returnvalue 0)
        (if (== `Ennemy Heart Emplacement` 2)
          (`KismetSystemLibrary.PrintString` "Critique")
          (set `self.Ennemy_Data` (make `/Game/Structure/ST_Ennemie_Data` (- _pv (* `Native Damage` 2)) `Ennemy Heart Emplacement` `Nbr Of Shield (Emplacement 1)` `Nbr Of Shield (Emplacement 2)` _returnvalue))
          (else
            (`KismetSystemLibrary.PrintString` "Normal")
            (bind _output_get (set `self.Ennemy_Data` (make `/Game/Structure/ST_Ennemie_Data` (- _pv `Native Damage`) `Ennemy Heart Emplacement` `Nbr Of Shield (Emplacement 1)` `Nbr Of Shield (Emplacement 2)` _returnvalue)))
            (`KismetSystemLibrary.PrintString` (`KismetStringLibrary.Conv_IntToString` (break `/Game/Structure/ST_Ennemie_Data` _output_get)))))
        (else
          (set `self.Ennemy_Data` (make `/Game/Structure/ST_Ennemie_Data` _pv `Ennemy Heart Emplacement` `Nbr Of Shield (Emplacement 1)` `Nbr Of Shield (Emplacement 2)` _returnvalue))))
      (return))))

(fn `Emplacement 1 Attacked`
  (params (`Number Of Projectile` :type Integer) (`Native Damage` :type Integer) (`Number Of Shield That Can Be Broken` :type Integer) (`Can deal damage through shield ?` :type Boolean) (` Damage added per destroyed shield` :type Integer) (`Can Deal Passive Damage ?` :type Boolean) (`Passive Damage` :type Integer) (`Ennemy HP` :type Integer) (`Ennemy Heart Emplacement` :type Integer) (`Nbr Of Shield (Emplacement 1)` :type Integer) (`Nbr Of Shield (Emplacement 2)` :type Integer) (`Nbr Of Shield (Emplacement 3)` :type Integer))
  (bind (_pv _heartemplacement _nbrofshieldemplacement1 _nbrofshieldemplacement2 _nbrofshieldemplacement3) (break `/Game/Structure/ST_Ennemie_Data` (`self.Ennemy_Data`)))
  (bind _returnvalue (`KismetMathLibrary.Clamp` (- `Nbr Of Shield (Emplacement 1)` `Number Of Shield That Can Be Broken`) 0 5))
  (`|ExecutionSequence` :!label _label
    (:`then_0`
      (if (== _returnvalue 0)
        (if (== `Ennemy Heart Emplacement` 0)
          (`KismetSystemLibrary.PrintString` "Critique")
          (set `self.Ennemy_Data` (make `/Game/Structure/ST_Ennemie_Data` (- `Ennemy HP` (* `Native Damage` 2)) `Ennemy Heart Emplacement` _returnvalue `Nbr Of Shield (Emplacement 2)` `Nbr Of Shield (Emplacement 3)`))
          (else
            (`KismetSystemLibrary.PrintString` "Normal")
            (set `self.Ennemy_Data` (make `/Game/Structure/ST_Ennemie_Data` (- `Ennemy HP` `Native Damage`) `Ennemy Heart Emplacement` _returnvalue `Nbr Of Shield (Emplacement 2)` `Nbr Of Shield (Emplacement 3)`))))
        (else
          (set `self.Ennemy_Data` (make `/Game/Structure/ST_Ennemie_Data` `Ennemy HP` `Ennemy Heart Emplacement` _returnvalue `Nbr Of Shield (Emplacement 2)` `Nbr Of Shield (Emplacement 3)`)))))
    (:`then_1`
      (if `Can deal damage through shield ?`
        (set `self.Ennemy_Data` (make `/Game/Structure/ST_Ennemie_Data` (- _pv (* ` Damage added per destroyed shield` `Nbr Of Shield (Emplacement 1)`)) _heartemplacement _nbrofshieldemplacement1 _nbrofshieldemplacement2 _nbrofshieldemplacement3))))
    (:`then_2`
      (if `Can Deal Passive Damage ?`
        (set `self.Passiv Damage ?` true)
        (set `self.Passiv Damage` `Passive Damage`))
      (bind _result (`/Engine/EditorBlueprintResources/StandardMacros.DecrementInt` `Number Of Projectile`)
        (:`  `
          (if (== _result 0)
            (return)
            (else
              (goto _label))))))))

(fn `Emplacement 2 Attacked`
  (params (`Number Of Projectile` :type Integer) (`Native Damage` :type Integer) (`Number Of Shield That Can Be Broken` :type Integer) (`Can deal damage through shield ?` :type Boolean) (` Damage added per destroyed shield` :type Integer) (`Can Deal Passive Damage ?` :type Boolean) (`Passive Damage` :type Integer) (`Ennemy HP` :type Integer) (`Ennemy Heart Emplacement` :type Integer) (`Nbr Of Shield (Emplacement 1)` :type Integer) (`Nbr Of Shield (Emplacement 2)` :type Integer) (`Nbr Of Shield (Emplacement 3)` :type Integer))
  (bind (_pv _heartemplacement _nbrofshieldemplacement1 _nbrofshieldemplacement2 _nbrofshieldemplacement3) (break `/Game/Structure/ST_Ennemie_Data` (`self.Ennemy_Data`)))
  (bind _returnvalue (`KismetMathLibrary.Clamp` (- `Nbr Of Shield (Emplacement 2)` `Number Of Shield That Can Be Broken`) 0 5))
  (`|ExecutionSequence` :!label _label
    (:`then_0`
      (if (== _returnvalue 0)
        (if (== `Ennemy Heart Emplacement` 1)
          (`KismetSystemLibrary.PrintString` "Critique")
          (set `self.Ennemy_Data` (make `/Game/Structure/ST_Ennemie_Data` (- `Ennemy HP` (* `Native Damage` 2)) `Ennemy Heart Emplacement` `Nbr Of Shield (Emplacement 1)` _returnvalue `Nbr Of Shield (Emplacement 3)`))
          (else
            (`KismetSystemLibrary.PrintString` "Normal")
            (set `self.Ennemy_Data` (make `/Game/Structure/ST_Ennemie_Data` (- `Ennemy HP` `Native Damage`) 0 `Nbr Of Shield (Emplacement 1)` _returnvalue `Nbr Of Shield (Emplacement 3)`))))
        (else
          (set `self.Ennemy_Data` (make `/Game/Structure/ST_Ennemie_Data` `Ennemy HP` `Ennemy Heart Emplacement` `Nbr Of Shield (Emplacement 1)` _returnvalue `Nbr Of Shield (Emplacement 3)`)))))
    (:`then_1`
      (if `Can deal damage through shield ?`
        (set `self.Ennemy_Data` (make `/Game/Structure/ST_Ennemie_Data` (- _pv (* ` Damage added per destroyed shield` `Nbr Of Shield (Emplacement 2)`)) _heartemplacement _nbrofshieldemplacement1 _nbrofshieldemplacement2 _nbrofshieldemplacement3))))
    (:`then_2`
      (if `Can Deal Passive Damage ?`
        (set `self.Passiv Damage ?` true)
        (set `self.Passiv Damage` `Passive Damage`))
      (bind _result (`/Engine/EditorBlueprintResources/StandardMacros.DecrementInt` `Number Of Projectile`)
        (:`  `
          (if (== _result 0)
            (return)
            (else
              (goto _label))))))))

(fn `Emplacement 3 Attacked`
  (params (`Number Of Projectile` :type Integer) (`Native Damage` :type Integer) (`Number Of Shield That Can Be Broken` :type Integer) (`Can deal damage through shield ?` :type Boolean) (` Damage added per destroyed shield` :type Integer) (`Can Deal Passive Damage ?` :type Boolean) (`Passive Damage` :type Integer) (`Ennemy HP` :type Integer) (`Ennemy Heart Emplacement` :type Integer) (`Nbr Of Shield (Emplacement 1)` :type Integer) (`Nbr Of Shield (Emplacement 2)` :type Integer) (`Nbr Of Shield (Emplacement 3)` :type Integer))
  (bind (_pv _heartemplacement _nbrofshieldemplacement1 _nbrofshieldemplacement2 _nbrofshieldemplacement3) (break `/Game/Structure/ST_Ennemie_Data` (`self.Ennemy_Data`)))
  (bind _returnvalue (`KismetMathLibrary.Clamp` (- `Nbr Of Shield (Emplacement 3)` `Number Of Shield That Can Be Broken`) 0 5))
  (`|ExecutionSequence` :!label _label
    (:`then_0`
      (if (== _returnvalue 0)
        (if (== `Ennemy Heart Emplacement` 2)
          (`KismetSystemLibrary.PrintString` "Critique")
          (set `self.Ennemy_Data` (make `/Game/Structure/ST_Ennemie_Data` (- `Ennemy HP` (* `Native Damage` 2)) `Ennemy Heart Emplacement` `Nbr Of Shield (Emplacement 1)` `Nbr Of Shield (Emplacement 2)` _returnvalue))
          (else
            (`KismetSystemLibrary.PrintString` "Normal")
            (set `self.Ennemy_Data` (make `/Game/Structure/ST_Ennemie_Data` (- `Ennemy HP` `Native Damage`) `Ennemy Heart Emplacement` `Nbr Of Shield (Emplacement 1)` `Nbr Of Shield (Emplacement 2)` _returnvalue))))
        (else
          (set `self.Ennemy_Data` (make `/Game/Structure/ST_Ennemie_Data` `Ennemy HP` `Ennemy Heart Emplacement` `Nbr Of Shield (Emplacement 1)` `Nbr Of Shield (Emplacement 2)` _returnvalue)))))
    (:`then_1`
      (if `Can deal damage through shield ?`
        (set `self.Ennemy_Data` (make `/Game/Structure/ST_Ennemie_Data` (- _pv (* ` Damage added per destroyed shield` `Nbr Of Shield (Emplacement 3)`)) _heartemplacement _nbrofshieldemplacement1 _nbrofshieldemplacement2 _nbrofshieldemplacement3))))
    (:`then_2`
      (if `Can Deal Passive Damage ?`
        (set `self.Passiv Damage ?` true)
        (set `self.Passiv Damage` `Passive Damage`))
      (bind _result (`/Engine/EditorBlueprintResources/StandardMacros.DecrementInt` `Number Of Projectile`)
        (:`  `
          (if (== _result 0)
            (return)
            (else
              (goto _label))))))))

(fn `UserConstructionScript`)